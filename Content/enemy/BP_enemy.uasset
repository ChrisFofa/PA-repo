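; Zombie enemy character that spots and chases the player, takes damage and ragdolls at zero health.
; PawnSensing sets blackboard flags, with a one-time scream before movement speed is raised.
; Attack sphere-traces ahead and plays a random montage without applying damage here.
; Caught and cursed events incapacitate an unaware enemy and cut off its sight response, while stagger briefly halts movement during a hit reaction.
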(event OnSeePawn(PawnSensing)
  (params (Pawn :type Pawn%20Object%20Reference))
  ;[1 1 1] chase player
  (Utilities|Casting|CastToBP_ThirdPersonCharacter Pawn)
  (AI|Components|Blackboard|SetValueasBool (AI|GetBlackboard (AI|GetAIController self)) (Utilities|Name|MakeLiteralName "has seen player") true)
  (Utilities|FlowControl|DoOnce false
    (:Completed
      (Pawn|Components|CharacterMovement|DisableMovement (Variables|Character|GetCharacterMovement))
      (bind _returnvalue (Animation|PlayAnimMontage "/Game/enemy/EnemyAnimations/zombie_anims/Zombie_Scream_Montage.Zombie_Scream_Montage" 1.0 "None"))
      (Utilities|FlowControl|Delay _returnvalue)
      (Pawn|Components|CharacterMovement|SetMovementMode (Variables|Character|GetCharacterMovement) "MOVE_Walking" 0)
      (Variables|/Script/Engine.CharacterMovementComponent|SetMaxWalkSpeed (Variables|Character|GetCharacterMovement) 4.5e+02)
      (AI|Components|Blackboard|SetValueasBool (AI|GetBlackboard (AI|GetAIController self)) (Utilities|Name|MakeLiteralName "is caught") false))))

(event Custom|attack%20player
  (bind _returnvalue (Transformation|GetActorLocation))
  (bind _attack_animations (Variables|Default|Getattack%20animations))
  (bind (_outhit _returnvalue_2) (Collision|SphereTraceForObjects _returnvalue (+ _returnvalue (* (Math|Vector|GetForwardVector (Transformation|GetActorRotation)) 5e+01)) 1e+01 (Utilities|Array|MakeArray "ObjectTypeQuery3") false 0 "None"))
  (if _returnvalue_2
    (Utilities|Casting|CastToBP_ThirdPersonCharacter (.HitActor (Collision|BreakHitResult _outhit)))
    (Animation|PlayAnimMontage (Utilities|Array|Get(acopy) _attack_animations (Math|Random|RandomInteger (Utilities|Array|Length _attack_animations))) 1.0 "None")))

(event Custom|is%20caught
  (if (not (ScalableFloat|GetValueasBool (AI|GetBlackboard (AI|GetAIController self)) (Utilities|Name|MakeLiteralName "has seen player")))
    (AI|Components|Blackboard|SetValueasBool (AI|GetBlackboard (AI|GetAIController self)) (Utilities|Name|MakeLiteralName "is caught") true)
    (EventDispatchers|UnbindallEventsfromOnSeePawn (Variables|Default|GetPawnSensing))
    (Pawn|Components|CharacterMovement|DisableMovement (Variables|Character|GetCharacterMovement))
    (Animation|Montage|PlayMontage (Variables|Character|GetMesh) "/Game/enemy/EnemyAnimations/zombie_anims/Terrified_Montage.Terrified_Montage" 1.0 0.5)))

(event Custom|cursed
  (if (not (ScalableFloat|GetValueasBool (AI|GetBlackboard (AI|GetAIController self)) (Utilities|Name|MakeLiteralName "has seen player")))
    (AI|Components|Blackboard|SetValueasBool (AI|GetBlackboard (AI|GetAIController self)) (Utilities|Name|MakeLiteralName "is caught") true)
    (Components|DestroyComponent (Variables|Default|GetPawnSensing))
    (Pawn|Components|CharacterMovement|DisableMovement (Variables|Character|GetCharacterMovement))
    (Animation|PlayAnimMontage "/Game/enemy/EnemyAnimations/zombie_anims/Being_Electrocuted_Montage.Being_Electrocuted_Montage" 1.0 "None")))

(event Custom|stager
  (Pawn|Components|CharacterMovement|DisableMovement (Variables|Character|GetCharacterMovement))
  (bind _returnvalue (Animation|PlayAnimMontage "/Game/enemy/EnemyAnimations/zombie_anims/Zombie_Reaction_Hit__1__Montage.Zombie_Reaction_Hit__1__Montage" 1.5 "None"))
  (Utilities|FlowControl|Delay _returnvalue)
  (Pawn|Components|CharacterMovement|SetMovementMode (Variables|Character|GetCharacterMovement) "MOVE_Walking" 0))

(event EventBeginPlay
  (Variables|Default|Setcurrent%20health (Variables|Default|Getmax%20health))
  (bind _aswb_enemy_health (Utilities|Casting|CastToWB_EnemyHealth (UserInterface|GetUserWidgetObject (Variables|Default|Gethealthbar))))
  (Default|EnemyHealthbarInfo _aswb_enemy_health (Variables|Default|Getcurrent%20health) (Variables|Default|Getmax%20health)))

(event Game|Damage|EventAnyDamage
  (params (Damage :type Float%20%28single-precision%29) (DamageType :type Damage%20Type%20Object%20Reference) (InstigatedBy :type Controller%20Object%20Reference) (DamageCauser :type Actor%20Object%20Reference))
  (bind _output_get (Variables|Default|Setcurrent%20health (- (Variables|Default|Getcurrent%20health) Damage)))
  (Development|PrintString (Utilities|String|ToString(Float) _output_get))
  (bind _aswb_enemy_health (Utilities|Casting|CastToWB_EnemyHealth (UserInterface|GetUserWidgetObject (Variables|Default|Gethealthbar))))
  (Default|EnemyHealthbarInfo _aswb_enemy_health (Variables|Default|Getcurrent%20health) (Variables|Default|Getmax%20health))
  ;[1 1 1] kills player if heaslth is 0
  (if (<= (Variables|Default|Getcurrent%20health) 0.0)
    (Physics|SetSimulatePhysics (Variables|Character|GetMesh) true)))

(fn ConstructionScript)